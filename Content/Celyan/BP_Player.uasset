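; BP_Player is a player Blueprint with movement, look, jump, climbing and interaction.
; Custom gravity and timeline-driven jumps use vertical movement input, with a downward ground trace setting the inverted-named IsFalling and re-arming jump after a delay.
; Camera box traces show an interaction prompt and message hit actors on F.
; Pressing jump while off the ground hands climbing to a traced climbable, otherwise jumps and sets IsFlying, which changes movement scale.
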(event `EnhancedInput|/Game/Input/Actions/IA_Move`
  (params (ActionValue :type "Vector2D Structure") (ElapsedSeconds :type "Float (double-precision)") (TriggeredSeconds :type "Float (double-precision)") (InputAction :type "InputAction Object Reference" :default "/Game/Input/Actions/IA_Move.IA_Move"))
  (bind (_returnvalue_roll _returnvalue_pitch _returnvalue_yaw) (`KismetMathLibrary.BreakRotator` (`self.K2_GetActorRotation`)))
  (bind (_returnvalue_roll_2 _returnvalue_pitch_2 _returnvalue_yaw_2) (`KismetMathLibrary.BreakRotator` (`self.K2_GetActorRotation`)))
  (:`Triggered`
    (set `self.Action Value X` ActionValue_X)
    (set `self.Action Value Y` ActionValue_Y)
    (`self.AddMovementInput` (`KismetMathLibrary.GetForwardVector` (`KismetMathLibrary.MakeRotator` _returnvalue_roll 0.0 _returnvalue_yaw)) (`KismetMathLibrary.SelectFloat` ActionValue_X (/ ActionValue_X 1.5) (not (`self.IsFlying`))))
    (`self.AddMovementInput` (`KismetMathLibrary.GetRightVector` (`KismetMathLibrary.MakeRotator` _returnvalue_roll_2 0.0 _returnvalue_yaw_2)) (`KismetMathLibrary.SelectFloat` ActionValue_Y (/ ActionValue_Y 1.5) (not (`self.IsFlying`))))))

(event `Print`
  (params (String :type String))
  (`KismetSystemLibrary.PrintString` String true true (struct :`G` 0.66 :`B` 1.0 :`A` 1.0) 0.0))

(event `EnhancedInput|/Game/Input/Actions/IA_Look`
  (params (ActionValue :type "Vector2D Structure") (ElapsedSeconds :type "Float (double-precision)") (TriggeredSeconds :type "Float (double-precision)") (InputAction :type "InputAction Object Reference" :default "/Game/Input/Actions/IA_Look.IA_Look"))
  (:`Triggered`
    (`self.AddControllerYawInput` ActionValue_X)
    (`self.AddControllerPitchInput` ActionValue_Y)))

(event `self.ReceiveTick`
  (params (DeltaSeconds :type "Float (single-precision)"))
  (`self.GroundDetection`)
  (`self.CanInteractUI`)
  (`self.Print` (`KismetStringLibrary.Conv_DoubleToString` (`self.ValueJump`)))
  (`self.RaycastDetection`))

(event `CanInteractUI`
  (bind _widgetref (`self.WidgetRef`))
  (bind _camera (`self.Camera`))
  (bind _returnvalue (`SceneComponent.K2_GetComponentLocation` _camera))
  (bind (_outhit _returnvalue_2) (`KismetSystemLibrary.BoxTraceSingleForObjects` _returnvalue (+ (* (`KismetMathLibrary.GetForwardVector` (`SceneComponent.K2_GetComponentRotation` _camera)) (`self.LenghtRaycast`)) _returnvalue) (20.0 20.0 20.0) (struct) (`self.ObjectInteractHit`)))
  (if _returnvalue_2
    (if (not (`self.HasWidget`))
      (bind _returnvalue_3 (`|CreateWidget` "/Game/FirstPerson/Blueprints/WB/WB_Interaction.WB_Interaction_C" null "Press F To Interact"))
      (`UserWidget.AddToViewport` _returnvalue_3 0)
      (bind _output_get (set `self.WidgetRef` _returnvalue_3))
      (message `/Game/FirstPerson/Blueprints/BPI_Interact.Interact_UI` (`.HitActor` (`GameplayStatics.BreakHitResult` _outhit)) _output_get)
      (set `self.HasWidget` true))
    (else
      (`/Engine/EditorBlueprintResources/StandardMacros.IsValid` _widgetref
        (:`Is Valid`
          (`Widget.RemoveFromParent` _widgetref)
          (set `self.HasWidget` false))))))

(event `Key|F`
  (params (Key :type "Key Structure"))
  (bind _camera (`self.Camera`))
  (bind _returnvalue (`SceneComponent.K2_GetComponentLocation` _camera))
  (:`Pressed`
    (bind _outhit (`KismetSystemLibrary.BoxTraceSingleForObjects` _returnvalue (+ (* (`KismetMathLibrary.GetForwardVector` (`SceneComponent.K2_GetComponentRotation` _camera)) (`self.LenghtRaycast`)) _returnvalue) (20.0 20.0 20.0) (struct) (`self.ObjectInteractHit`)))
    (message `/Game/FirstPerson/Blueprints/BPI_Interact.Interact` (`.HitActor` (`GameplayStatics.BreakHitResult` _outhit)))))

(event `EnhancedInput|/Game/Input/Actions/IA_Jump`
  (params (ActionValue :type Boolean) (ElapsedSeconds :type "Float (double-precision)") (TriggeredSeconds :type "Float (double-precision)") (InputAction :type "InputAction Object Reference" :default "/Game/Input/Actions/IA_Jump.IA_Jump"))
  (bind _camera (`self.Camera`))
  (bind _returnvalue (`SceneComponent.K2_GetComponentLocation` _camera))
  (:`Started`
    (`/Engine/EditorBlueprintResources/StandardMacros.DoOnce` false :!label _label
      (:`Completed`
        (bind (_outhit _returnvalue_2) (`KismetSystemLibrary.BoxTraceSingleForObjects` :`Start` _returnvalue :`End` (+ (* (`KismetMathLibrary.GetForwardVector` (`SceneComponent.K2_GetComponentRotation` _camera)) (`self.LenghtRaycast`)) _returnvalue) :`HalfSize` (10.0 10.0 20.0) :`ObjectTypes` (`self.ObjectClimb`) :`DrawDebugType` "ForDuration"))
        (if (and (not (`self.IsFalling`)) _returnvalue_2)
          (message `/Game/FirstPerson/Blueprints/BPI_Interact.EventOnClimb` (`.HitActor` (`GameplayStatics.BreakHitResult` _outhit)) self)
          (else
            (set `self.IsJumping` true)
            (set `self.IsFlying` true)
            (bind (_direction _newtrack_0) (`Timeline|JumpForce` :!via `PlayFromStart`)
              (:`Update`
                (bind _output_get (set `self.ValueJump` (* (* _newtrack_0 (`self.JumpPower`)) (`GameplayStatics.GetWorldDeltaSeconds`))))
                (`self.AddMovementInput` (0.0 0.0 1.0) _output_get))
              (:`Finished`
                (set `self.IsJumping` false)))))))))

(event `ResetDoJump`
  (`KismetSystemLibrary.Delay` 1.0)
  (goto _label :!via `Reset`))

(event `RaycastDetection`
  (bind _box (`self.Box`))
  (bind _returnvalue (`SceneComponent.K2_GetComponentLocation` _box))
  (if (and (not (`self.IsClimbing`)) (not (`self.IsJumping`)))
    (bind (_outhit _returnvalue_2) (`KismetSystemLibrary.BoxTraceSingleForObjects` :`Start` _returnvalue :`End` (+ (* (`KismetMathLibrary.GetUpVector` (`SceneComponent.K2_GetComponentRotation` _box)) -100.0) _returnvalue) :`HalfSize` (5.0 5.0 1.0) :`ObjectTypes` (`self.GroundObject`) :`DrawDebugType` "ForOneFrame"))
    (set `self.IsFalling` _returnvalue_2)))

(event `GroundDetection`
  (if (`self.IsFalling`)
    (`self.ResetDoJump`)
    (set `self.Scale Value Gravity` 0.0)
    (else
      (bind _output_get (set `self.Scale Value Gravity` (- (`self.Scale Value Gravity`) 0.0981)))
      (`self.AddMovementInput` (0.0 0.0 1.0) (`KismetMathLibrary.FClamp` _output_get -4.0 0.0)))))

(fn `UserConstructionScript`)